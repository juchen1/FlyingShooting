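; BP_PlayerDragon is the player-controlled flying dragon character for the FlyingShooting game.
; On BeginPlay it adds its Enhanced Input mapping context, with move input driving movement along control-yaw forward and right vectors and look input scaled by mouse sensitivity.
; A hard-wired Space Bar key doubles max fly speed while held.
; Tick is empty, and a speed debug print is left disconnected.
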(event `self.ReceiveBeginPlay`
  (`EnhancedInputSubsystemInterface.AddMappingContext` (pcsubsystem `EnhancedInputLocalPlayerSubsystem` (`GameplayStatics.GetPlayerController` 0)) "/Game/FlyingShooting/Input/IMC_PlayerDragon.IMC_PlayerDragon" 0 (struct)))

(event `EnhancedInput|/Game/FlyingShooting/Input/IA_PlayerDragonMove`
  (params (ActionValue :type "Vector2D Structure") (ElapsedSeconds :type "Float (double-precision)") (TriggeredSeconds :type "Float (double-precision)") (InputAction :type "InputAction Object Reference" :default "/Game/FlyingShooting/Input/IA_PlayerDragonMove.IA_PlayerDragonMove"))
  (bind (_returnvalue_roll _returnvalue_pitch _returnvalue_yaw) (`KismetMathLibrary.BreakRotator` (`self.GetControlRotation`)))
  (bind (_returnvalue_x _returnvalue_y) (`KismetMathLibrary.BreakVector2D` (`KismetMathLibrary.Normal2D` ActionValue)))
  (bind _returnvalue (`KismetMathLibrary.MakeRotator` 0.0 0.0 _returnvalue_yaw))
  (:`Triggered`
    (`self.AddMovementInput` (`KismetMathLibrary.GetRightVector` _returnvalue) _returnvalue_x)
    (`self.AddMovementInput` (`KismetMathLibrary.GetForwardVector` _returnvalue) _returnvalue_y)))

(event `EnhancedInput|/Game/FlyingShooting/Input/IA_PlayerDragonLook`
  (params (ActionValue :type "Vector2D Structure") (ElapsedSeconds :type "Float (double-precision)") (TriggeredSeconds :type "Float (double-precision)") (InputAction :type "InputAction Object Reference" :default "/Game/FlyingShooting/Input/IA_PlayerDragonLook.IA_PlayerDragonLook"))
  (bind (_returnvalue_x _returnvalue_y) (`KismetMathLibrary.BreakVector2D` (* ActionValue (`self.MouseSensivity`))))
  (:`Triggered`
    (`self.AddControllerYawInput` _returnvalue_x)
    (`self.AddControllerPitchInput` _returnvalue_y)))

(event `Key|SpaceBar`
  (params (Key :type "Key Structure"))
  (bind _charactermovement (`self.CharacterMovement`))
  (:`Pressed`
    (set `CharacterMovementComponent.MaxFlySpeed` 6000.0 _charactermovement))
  (:`Released`
    (set `CharacterMovementComponent.MaxFlySpeed` 3000.0 _charactermovement)))

(event `self.ReceiveTick`
  (params (DeltaSeconds :type "Float (single-precision)")))

(fn `UserConstructionScript`)