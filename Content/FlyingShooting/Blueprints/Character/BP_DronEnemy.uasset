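; Enemy drone for a flying shooter that turns smoothly toward player 0's pawn every tick and is destroyed when damage drains its HP.
; A self-calling MoveNPC loop jumps it by a random horizontal offset every five seconds, then fires from left and right rifle sockets.
; Each shot spawns a BP_BlasterBeam with burst effect and sound.
; Damage also broadcasts HP changes; StoreTargetPawn is an empty stub.
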(event `self.ReceiveBeginPlay`
  (`self.StoreTargetPawn`)
  (`self.MoveNPC`))

(event `self.ReceiveAnyDamage`
  (params (Damage :type "Float (single-precision)") (DamageType :type "DamageType Object Reference") (InstigatedBy :type "Controller Object Reference") (DamageCauser :type "Actor Object Reference"))
  (bind _output_get (set `self.HP` (- (`self.HP`) Damage)))
  (`self.OnHPChange` _output_get)
  (if (<= _output_get 0.0)
    (`self.K2_DestroyActor`)))

(event `self.ReceiveTick`
  (params (DeltaSeconds :type "Float (single-precision)"))
  ;[0.08501 0.1395 0.15 0.5] Interpolate Rotation to TargetPawn
  (`self.InterpRotation` DeltaSeconds (`self.RotationInterpSpeed`)))

(event `MoveNPC`
  (`self.K2_AddActorWorldOffset` (`KismetMathLibrary.MakeVector` (`KismetMathLibrary.RandomFloatInRange` -1000.0 1000.0) (`KismetMathLibrary.RandomFloatInRange` -1000.0 1000.0)))
  (`KismetSystemLibrary.Delay` 5.0)
  (`self.MoveNPC`)
  (`self.SpawnBlasterBeam` (`self.RifleSocketName_L`))
  (`self.SpawnBlasterBeam` (`self.RifleSocketName_R`)))

(fn `FindTargetRotation`
  (returns (TargetRotation :type "Rotator Structure"))
  (return (`KismetMathLibrary.FindLookAtRotation` (`self.K2_GetActorLocation`) (`self.K2_GetActorLocation` (`GameplayStatics.GetPlayerPawn` 0)))))

(fn `InterpRotation`
  (params (DeltaTime :type "Float (single-precision)") (InterpSpeed :type "Float (double-precision)"))
  (`self.K2_SetActorRotation` (`KismetMathLibrary.RInterpTo` (`self.K2_GetActorRotation`) (`self.FindTargetRotation`) DeltaTime InterpSpeed)))

(fn `SpawnBlasterBeam`
  (params (SocketName :type Name))
  (bind (_returnvalue_location _returnvalue_rotation) (`KismetMathLibrary.BreakTransform` (`SceneComponent.GetSocketTransform` (`self.BotMesh`) (`local.SocketName`) "RTS_World")))
  (`|SpawnActorFromClass` "/Game/FlyingShooting/Blueprints/Character/BP_BlasterBeam.BP_BlasterBeam_C" (`SceneComponent.GetSocketTransform` (`self.BotMesh`) (`local.SocketName`) "RTS_World") "Undefined" "MultiplyWithRoot" null null)
  (`NiagaraFunctionLibrary.SpawnSystemAtLocation` "/Game/FlyingShooting/FX/NS_BeamBurst.NS_BeamBurst" _returnvalue_location _returnvalue_rotation)
  (`GameplayStatics.PlaySoundAtLocation` "/Game/FlyingShooting/Sound/SFX_EnergyRifle.SFX_EnergyRifle" _returnvalue_location (struct) 1.0 1.0 0.0 null null null null))

(fn `StoreTargetPawn`)

(fn `UserConstructionScript`)