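; Player controller for the dragon in a flying shooting game, linking the possessed pawn's health to the HUD.
; On BeginPlay it restricts camera view pitch to a narrow range from level to slightly downward.
; On possession it binds to the BP_PlayerDragon HP change event and pushes the current HP to the Hud_Play widget.
; GetLife is a stub returning zero.
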(event `self.ReceiveBeginPlay`
  (bind _returnvalue (`GameplayStatics.GetPlayerCameraManager` 0))
  (set `PlayerCameraManager.ViewPitchMin` -10.0 _returnvalue)
  (set `PlayerCameraManager.ViewPitchMax` 0.0 _returnvalue))

(event `self.ReceivePossess`
  (params (PossessedPawn :type "Pawn Object Reference"))
  (bind _asbp_player_dragon (cast `/Game/FlyingShooting/Blueprints/Character/BP_PlayerDragon` PossessedPawn))
  (add `/Game/FlyingShooting/Blueprints/Character/BP_PlayerDragon.OnHPChange` _asbp_player_dragon (delegate `UI_Update`))
  (`self.UI_Update` (`/Game/FlyingShooting/Blueprints/Character/BP_PlayerDragon.HP` _asbp_player_dragon)))

(event `UI_Update`
  (params (CurrentHP :type "Float (double-precision)"))
  (bind _ashud_play (cast `/Game/FlyingShooting/Blueprints/Frameworks/Hud_Play` (`self.GetHUD`)))
  (bind _ui_play (`/Game/FlyingShooting/Blueprints/Frameworks/Hud_Play.UI_Play` _ashud_play))
  (`/Engine/EditorBlueprintResources/StandardMacros.IsValid` _ui_play
    (:`Is Valid`
      (`/Game/FlyingShooting/UI/WBP_GamePlayTime.OnHPUPdate` _ui_play CurrentHP))))

(fn `GetLife`
  (returns (Life :type "Float (double-precision)"))
  (return 0.0))

(fn `UserConstructionScript`)