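; Game mode for the dragon flying-shooter level that tracks enemies and ends the match.
; It keeps a running enemy total and declares a clear when it reaches zero, while game over and clear both show the clear board on the play HUD.
; On begin play it caches the level's BP_EnemyPool and hands out pooled drone teleport actors at a given transform.
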(event `self.ReceiveBeginPlay`
  (bind _outactors (`GameplayStatics.GetAllActorsOfClass` "/Game/FlyingShooting/Blueprints/Enemy/BP_EnemyPool.BP_EnemyPool_C"))
  (set `self.EnemyPool` (`|GetArrayItem` _outactors)))

(event `/Game/FlyingShooting/Blueprints/Interface/BPI_GameEnd.GameOver`
  (bind _ashud_play (cast `/Game/FlyingShooting/Blueprints/Frameworks/Hud_Play` (`PlayerController.GetHUD` (`GameplayStatics.GetPlayerController` 0))))
  (`/Game/FlyingShooting/UI/WBP_GamePlayTime.ShowClearBoard` (`/Game/FlyingShooting/Blueprints/Frameworks/Hud_Play.UI_Play` _ashud_play) true false))

(event `/Game/FlyingShooting/Blueprints/Interface/BPI_GameEnd.GameClear`
  (bind _ashud_play (cast `/Game/FlyingShooting/Blueprints/Frameworks/Hud_Play` (`PlayerController.GetHUD` (`GameplayStatics.GetPlayerController` 0))))
  (bind _ui_play (`/Game/FlyingShooting/Blueprints/Frameworks/Hud_Play.UI_Play` _ashud_play))
  (`/Engine/EditorBlueprintResources/StandardMacros.IsValid` _ui_play
    (:`Is Valid`
      (`/Game/FlyingShooting/UI/WBP_GamePlayTime.ShowClearBoard` _ui_play true true))))

(event `/Game/FlyingShooting/Blueprints/Enemy/BPI_EnemyManager.UpdateEnemyCount`
  (params (ChangeAmount :type Integer))
  (bind _output_get (set `self.TotalEnemies` (+ ChangeAmount (`self.TotalEnemies`))))
  (if (<= _output_get 0)
    (`/Game/FlyingShooting/Blueprints/Interface/BPI_GameEnd.GameClear`)))

(fn `CheckRemainingEnemies`
  (returns (RemainingCount :type Integer))
  (return (`self.TotalEnemies`)))

(fn `GetEnemyDroneTeleport`
  (params (SpawnTransform :type "Transform Structure"))
  (returns (NewEnemy :type "/Game/FlyingShooting/Blueprints/Enemy/BP_DroneBase Object Reference"))
  (bind _enemypool (`self.EnemyPool`))
  (`/Engine/EditorBlueprintResources/StandardMacros.IsValid` _enemypool
    (:`Is Valid`
      (bind _newobject (`/Game/FlyingShooting/Blueprints/ObjectPool/AC_ObjectPool.GetObject` (`/Game/FlyingShooting/Blueprints/Enemy/BP_EnemyPool.Pool_DroneTeleport` _enemypool) SpawnTransform))
      (bind _asbp_drone_teleport (cast `/Game/FlyingShooting/Blueprints/Enemy/BP_DroneTeleport` _newobject))
      (return _asbp_drone_teleport))))

(fn `UserConstructionScript`)