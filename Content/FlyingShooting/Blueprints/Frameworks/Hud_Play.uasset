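; Play-mode HUD for the flying shooting game that runs the start-screen input and hands off to gameplay.
; On BeginPlay it shows the start widget in UI-only input mode and binds to its OnInputEnd dispatcher.
; When input ends, it restores game-only input, stores the entered dragon HP and drone count, rebroadcasts them through OnInputEndReceived, and adds the play-time widget.
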(event `self.ReceiveBeginPlay`
  (bind _returnvalue (`|CreateWidget` "/Game/FlyingShooting/UI/WBP_GameStart.WBP_GameStart_C"))
  (bind _output_get (set `self.UI_Start` _returnvalue))
  (`UserWidget.AddToViewport` _output_get 0)
  (`WidgetBlueprintLibrary.SetInputMode_UIOnlyEx` (`GameplayStatics.GetPlayerController` 0) null "LockAlways" true)
  (add `/Game/FlyingShooting/UI/WBP_GameStart.OnInputEnd` (`self.UI_Start`) (delegate `OnInputEnd`)))

(event `OnInputEnd`
  (params (DragonHP :type "Float (double-precision)") (DroneCount :type Integer))
  (`WidgetBlueprintLibrary.SetInputMode_GameOnly` (`GameplayStatics.GetPlayerController` 0) true)
  (bind _output_get (set `self.Input Dragon HP` DragonHP))
  (bind _output_get_2 (set `self.Drone Num` DroneCount))
  (`self.OnInputEnd_Received` _output_get_2 _output_get)
  (bind _returnvalue (`|CreateWidget` "/Game/FlyingShooting/UI/WBP_GamePlayTime.WBP_GamePlayTime_C" (`GameplayStatics.GetPlayerController` 0)))
  (bind _output_get_3 (set `self.UI_Play` _returnvalue))
  (`UserWidget.AddToViewport` _output_get_3 0))

(fn `UserConstructionScript`)