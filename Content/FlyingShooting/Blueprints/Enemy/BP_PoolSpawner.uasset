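; BP_PoolSpawner places the enemy drones for the flying shooter, using the drone count received from the play HUD.
; On BeginPlay it binds SpawnDrone to Hud_Play's input-end event, whose DragonHP value it ignores.
; After a short delay, it loops per drone, messaging the game mode to update the enemy count and teleport a drone to a random XY position at fixed height, rather than spawning actors itself.
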(event `self.ReceiveBeginPlay`
  (bind _ashud_play (cast `/Game/FlyingShooting/Blueprints/Frameworks/Hud_Play` (`PlayerController.GetHUD` (`GameplayStatics.GetPlayerController` 0))))
  (bind _output_get (set `self.As Hud Play` _ashud_play))
  (add `/Game/FlyingShooting/Blueprints/Frameworks/Hud_Play.OnInputEnd_Received` _output_get (delegate `SpawnDrone`)))

(event `SpawnDrone`
  (params (DroneCount :type Integer) (DragonHP :type "Float (double-precision)"))
  (bind _output_get (set `self.NumberOfPool` DroneCount))
  (`KismetSystemLibrary.Delay` 0.2)
  (for _ (range _output_get)
    (bind _output_get_2 (set `self.Location` (`KismetMathLibrary.MakeVector` (`KismetMathLibrary.RandomFloatInRange` -3000.0 3000.0) (`KismetMathLibrary.RandomFloatInRange` -3000.0 3000.0) 500.0)))
    (message `/Game/FlyingShooting/Blueprints/Enemy/BPI_EnemyManager.UpdateEnemyCount` (`GameplayStatics.GetGameMode`) 1)
    (message `/Game/FlyingShooting/Blueprints/Enemy/BPI_GetEnemyDrone.GetEnemyDroneTeleport` (`GameplayStatics.GetGameMode`) (`KismetMathLibrary.MakeTransform` _output_get_2))))

(fn `UserConstructionScript`)