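; Teleporting drone enemy for the flying shooting game that jumps to nearby spots and fires blaster beams.
; On activation, MoveDrone starts a self-repeating delayed loop that applies a random horizontal offset every few seconds, firing from both rifle sockets shortly after each repeat jump.
; Tick interpolates rotation toward the target pawn.
; Damage reduces HP, broadcasts the change and destroys the drone at zero.
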(event `/Game/FlyingShooting/Blueprints/ObjectPool/BP_PoolingObject.OnActivate`
  (`self.MoveDrone`))

(event `self.ReceiveAnyDamage`
  (params (Damage :type "Float (single-precision)") (DamageType :type "DamageType Object Reference") (InstigatedBy :type "Controller Object Reference") (DamageCauser :type "Actor Object Reference"))
  (bind _output_get (set `self.HP_0` (- (`self.HP_0`) Damage)))
  (`self.OnHPChange` _output_get)
  (if (<= _output_get 0.0)
    (`self.K2_DestroyActor`)))

(event `self.ReceiveTick`
  (params (DeltaSeconds :type "Float (single-precision)"))
  ;[0.08501 0.1395 0.15 0.5] Interpolate Rotation to TargetPawn
  (`self.InterpRotation` DeltaSeconds (`self.RotationInterpSpeed_0`)))

(event `MoveDrone`
  (`self.K2_AddActorWorldOffset` (`KismetMathLibrary.MakeVector` (`KismetMathLibrary.RandomFloatInRange` -500.0 500.0) (`KismetMathLibrary.RandomFloatInRange` -500.0 500.0)))
  (`KismetSystemLibrary.Delay` 4.0)
  (`self.MoveDrone`)
  (`KismetSystemLibrary.Delay` 0.5)
  (`self.SpawnBlasterBeam` (`self.RifleSocketName_L`))
  (`self.SpawnBlasterBeam` (`self.RifleSocketName_R`)))

(fn `MoveNPC`)

(fn `StoreTargetPawn`)

(fn `UserConstructionScript`
  (`parent.UserConstructionScript`))